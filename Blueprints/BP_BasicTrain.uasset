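; Train actor made of a head, three locomotive parts and a tail, gathered into TrainParts by the construction script.
; RecalculateLocomotiveTransforms moves Loco1 and Loco2 to world transforms queried by index, leaving Loco3 untouched, and draws a debug line along Loco1's heading.
; AttachLevers snaps the head and tail levers onto two scene components, keeping world scale, and GetHead exposes the head part.
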(event `self.RecalculateLocomotiveTransforms`
  (bind _loco1 (`self.Loco1`))
  (bind _loco2 (`self.Loco2`))
  (bind _returnvalue (`SceneComponent.K2_GetComponentLocation` _loco1))
  (bind _returnvalue_2 (`self.GetLocomotiveWorldLocation` 1))
  (bind _returnvalue_3 (`self.GetLocomotiveWorldRotation` 1))
  (`SceneComponent.K2_SetWorldLocation` _loco1 _returnvalue_2 false false)
  (`SceneComponent.K2_SetWorldRotation` _loco1 _returnvalue_3 false false)
  (`KismetSystemLibrary.DrawDebugLine` _returnvalue (+ _returnvalue (* (`KismetMathLibrary.Conv_RotatorToVector` _returnvalue_3) 500.0)) (struct :`B` 1.0 :`A` 1.0) 0.0 5.0)
  (bind _returnvalue_4 (`self.GetLocomotiveWorldLocation` 2))
  (bind _returnvalue_5 (`self.GetLocomotiveWorldRotation` 2))
  (`SceneComponent.K2_SetWorldLocation` _loco2 _returnvalue_4 false false)
  (`SceneComponent.K2_SetWorldRotation` _loco2 _returnvalue_5 false false))

(fn `AttachLevers`
  (params (LeverHead :type "Actor Object Reference") (LeverTail :type "Actor Object Reference"))
  (`self.K2_AttachToComponent` LeverHead (`self.Scene2`) "None" "SnapToTarget" "SnapToTarget" "KeepWorld" true)
  (`self.K2_AttachToComponent` LeverTail (`self.Scene1`) "None" "SnapToTarget" "SnapToTarget" "KeepWorld" true))

(fn `GetHead`
  (returns (Head :type "StaticMeshComponent Object Reference"))
  (return (`self.Head`)))

(fn `UserConstructionScript`
  (set `self.TrainParts` (`|MakeArray` (`self.Head`) (`self.Loco1`) (`self.Loco2`) (`self.Loco3`) (`self.Tail`))))