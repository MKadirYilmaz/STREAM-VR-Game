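; Teleporter machine Blueprint that synchronizes its door animation with a teleport.
; Door events play the montage on the machine mesh, with ExecdoorAnim resuming it instead if already active.
; Montage notifies drive the sequence: when the doors close it pauses, calls ExecuteTeleport, then resumes after a short delay.
; The finish notify pauses the montage again, leaving it ready for ExecdoorAnim to resume.
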(event `self.ExecDoorAnimation`
  (params (DoorCondition :type Boolean))
  (bind _returnvalue (`SkeletalMeshComponent.GetAnimInstance` (`self.MachineMesh`)))
  (if DoorCondition
    (bind _notifyname (`|PlayMontage` (`self.MachineMesh`) "/Game/3D_Models/Teleporter/TeleporterDoorAnim.TeleporterDoorAnim" :!label _label)
      (:`OnNotifyBegin`
        (if (== _notifyname "DoorsClosed")
          (`AnimInstance.Montage_Pause` _returnvalue "/Game/3D_Models/Teleporter/TeleporterDoorAnim.TeleporterDoorAnim")
          (`self.ExecuteTeleport`)
          (`KismetSystemLibrary.Delay` 0.5)
          (`AnimInstance.Montage_Resume` _returnvalue "/Game/3D_Models/Teleporter/TeleporterDoorAnim.TeleporterDoorAnim")
          (elif (== _notifyname "AnimFinished")
            (`AnimInstance.Montage_Pause` _returnvalue "/Game/3D_Models/Teleporter/TeleporterDoorAnim.TeleporterDoorAnim")))))))

(event `Exec door Anim`
  (bind _returnvalue (`SkeletalMeshComponent.GetAnimInstance` (`self.MachineMesh`)))
  (if (`AnimInstance.Montage_IsActive` _returnvalue "/Game/3D_Models/Teleporter/TeleporterDoorAnim.TeleporterDoorAnim")
    (`AnimInstance.Montage_Resume` _returnvalue "/Game/3D_Models/Teleporter/TeleporterDoorAnim.TeleporterDoorAnim")
    (else
      (goto _label))))

(fn `UserConstructionScript`)