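; Ropeway Blueprint that lays spline meshes along the path of its Ropeway spline.
; The construction script adds one spline mesh per spline point, using local locations and tangents of that point and the next, then attaches it to the root.
; A SetupArrays event passes TiedTeleferics to SetTeleferics; BeginPlay and Tick contain no logic.
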(event `self.ReceiveBeginPlay`)

(event `self.ReceiveTick`
  (params (DeltaSeconds :type "Float (single-precision)")))

(event `self.SetupArrays`
  (`self.SetTeleferics` (`self.TiedTeleferics`)))

(fn `UserConstructionScript`
  (bind _ropeway (`self.Ropeway`))
  (for _index (range (`SplineComponent.GetNumberOfSplinePoints` (`self.Ropeway`)))
    (bind _returnvalue (`AddComponent|NODE_AddSplineMeshComponent-0`))
    (bind (_location _tangent) (`SplineComponent.GetLocationAndTangentAtSplinePoint` _ropeway _index "Local"))
    (bind (_location_2 _tangent_2) (`SplineComponent.GetLocationAndTangentAtSplinePoint` _ropeway (+ _index 1) "Local"))
    (`SplineMeshComponent.SetStartAndEnd` _returnvalue _location _tangent _location_2 _tangent_2 true)
    (`SceneComponent.K2_AttachToComponent` _returnvalue (`self.RootComponent`) "None" "KeepRelative" "KeepRelative" "KeepRelative" true)))