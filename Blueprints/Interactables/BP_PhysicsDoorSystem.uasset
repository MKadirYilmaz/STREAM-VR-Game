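; A grabbable interactable door whose handle and door mesh rotate to follow a grabber component, with a locked-state prompt.
; Look-at angles, clamped to set limits, drive handle roll and door yaw, and a separate event resets the door's yaw.
; Tick derives pulled and open states from those rotations and eases the handle back when not grabbed.
; When locked, a trigger zone shows text that turns toward the player.
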(event `self.ReceiveTick`
  (params (DeltaSeconds :type "Float (single-precision)"))
  (bind _doorhandle (`self.DoorHandle`))
  (bind (_relativerotation_roll _relativerotation_pitch _relativerotation_yaw) (`KismetMathLibrary.BreakRotator` (`SceneComponent.RelativeRotation` (`self.DoorMesh`))))
  (bind _relativerotation_roll_2 (`KismetMathLibrary.BreakRotator` (`SceneComponent.RelativeRotation` (`self.DoorHandle`))))
  (`|ExecutionSequence`
    (:`then_0`
      (`self.SetDoorBeingPulled` (> _relativerotation_roll_2 15.0)))
    (:`then_1`
      (`self.SetDoorOpenPosition` (> (`KismetMathLibrary.Abs` _relativerotation_yaw) 91.0)))
    (:`then_2`
      (if (`self.ShouldShowText`)
        (`self.RotateTextToPlayer`)))
    (:`then_3`
      (if (not (`self.GetIsGrabbing`))
        (`SceneComponent.K2_SetRelativeRotation` _doorhandle (`KismetMathLibrary.RInterpTo` (`SceneComponent.RelativeRotation` _doorhandle) (struct :`Yaw` 90.0) DeltaSeconds 3.0) false false)))))

(event `self.ReceiveBeginPlay`
  (set `self.GrabberComp` (`self.DoorAndHandleTarget`)))

(event `self.ReturnDoorToOriginalPositon`
  (bind _doormesh (`self.DoorMesh`))
  (bind (_relativerotation_roll _relativerotation_pitch) (`KismetMathLibrary.BreakRotator` (`SceneComponent.RelativeRotation` _doormesh)))
  (`SceneComponent.K2_SetRelativeRotation` _doormesh (`KismetMathLibrary.MakeRotator` _relativerotation_roll _relativerotation_pitch -90.0) false false))

(event `self.CalculateHandleRotation`
  (params (Grabber :type "SceneComponent Object Reference") (HandleMesh :type "StaticMeshComponent Object Reference"))
  (bind (_relativerotation_roll _relativerotation_pitch _relativerotation_yaw) (`KismetMathLibrary.BreakRotator` (`SceneComponent.RelativeRotation` HandleMesh)))
  (bind (_returnvalue_roll _returnvalue_pitch) (`KismetMathLibrary.BreakRotator` (`KismetMathLibrary.FindLookAtRotation` (`SceneComponent.K2_GetComponentLocation` HandleMesh) (`SceneComponent.K2_GetComponentLocation` Grabber))))
  (`SceneComponent.K2_SetRelativeRotation` HandleMesh (`KismetMathLibrary.MakeRotator` (`KismetMathLibrary.FClamp` (* _returnvalue_pitch -1.0) 0.0 40.0) _relativerotation_pitch _relativerotation_yaw) false false))

(event `self.CalculateDoorRotationForHand`
  (params (Grabber :type "SceneComponent Object Reference") (DoorStaticMesh :type "StaticMeshComponent Object Reference"))
  (bind (_relativerotation_roll _relativerotation_pitch) (`KismetMathLibrary.BreakRotator` (`SceneComponent.RelativeRotation` DoorStaticMesh)))
  (bind (_returnvalue_roll _returnvalue_pitch _returnvalue_yaw) (`KismetMathLibrary.BreakRotator` (`KismetMathLibrary.FindLookAtRotation` (`SceneComponent.RelativeLocation` DoorStaticMesh) (`SceneComponent.RelativeLocation` Grabber))))
  (`SceneComponent.K2_SetRelativeRotation` (`self.DoorMesh`) (`KismetMathLibrary.MakeRotator` _relativerotation_roll _relativerotation_pitch (`KismetMathLibrary.ClampAngle` (+ _returnvalue_yaw (`self.GetRotationDifference`)) 180.0 270.0)) false false)
  (`SceneComponent.K2_SetRelativeRotation` DoorStaticMesh (`KismetMathLibrary.MakeRotator` _relativerotation_roll _relativerotation_pitch (`KismetMathLibrary.ClampAngle` (+ _returnvalue_yaw (`self.GetRotationDifference`)) 180.0 270.0)) false false))

(event `self.DoorCloseZone.OnComponentBeginOverlap`
  (params (OverlappedComponent :type "PrimitiveComponent Object Reference") (OtherActor :type "Actor Object Reference") (OtherComp :type "PrimitiveComponent Object Reference") (OtherBodyIndex :type Integer) (bFromSweep :type Boolean) (SweepResult :type "HitResult Structure (by ref)"))
  (if (and (== OtherActor (`GameplayStatics.GetPlayerCharacter` 0)) (`self.GetIsLocked`))
    (`SceneComponent.SetVisibility` (`self.LockedText`) true false)
    (set `self.ShouldShowText` true)))

(event `self.DoorCloseZone.OnComponentEndOverlap`
  (params (OverlappedComponent :type "PrimitiveComponent Object Reference") (OtherActor :type "Actor Object Reference") (OtherComp :type "PrimitiveComponent Object Reference") (OtherBodyIndex :type Integer))
  (if (and (== OtherActor (`GameplayStatics.GetPlayerCharacter` 0)) (`self.GetIsLocked`))
    (`SceneComponent.SetVisibility` (`self.LockedText`) false false)
    (set `self.ShouldShowText` false)))

(fn `RotateTextToPlayer`
  (bind _lockedtext (`self.LockedText`))
  (bind (_returnvalue_roll _returnvalue_pitch) (`KismetMathLibrary.BreakRotator` (`SceneComponent.K2_GetComponentRotation` _lockedtext)))
  (bind (_returnvalue_roll_2 _returnvalue_pitch_2 _returnvalue_yaw) (`KismetMathLibrary.BreakRotator` (`KismetMathLibrary.FindLookAtRotation` (`SceneComponent.K2_GetComponentLocation` _lockedtext) (`self.K2_GetActorLocation` (`GameplayStatics.GetPlayerCharacter` 0)))))
  (`SceneComponent.K2_SetWorldRotation` _lockedtext (`KismetMathLibrary.MakeRotator` _returnvalue_roll_2 _returnvalue_pitch _returnvalue_yaw) false false))

(fn `UserConstructionScript`)