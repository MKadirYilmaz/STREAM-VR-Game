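; Grabbable lever actor whose handle angle becomes a lever value, hiding its Cube component at BeginPlay.
; CalculateLeverRotation aims the handle at the grabbing hand with a look-at in the actor's local XZ plane, clamped to a 100-degree pitch arc.
; Tick derives the value from the handle's forward-vector X, scaled to normalize that arc.
; Separate events reset the handle rotation or offset its pitch using the current value.
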(event `self.ResetLeverRotation`
  (`SceneComponent.K2_SetRelativeRotation` (`self.HandleMesh`) (struct :`Pitch` -90.0 :`Yaw` 2520.0 :`Roll` -360.0) false false))

(event `self.ReceiveBeginPlay`
  (`SceneComponent.SetVisibility` (`self.Cube`) false false))

(event `self.SetLeverPitchValue`
  (params (Value :type "Float (single-precision)"))
  (`SceneComponent.K2_AddLocalRotation` (`self.HandleMesh`) (`KismetMathLibrary.MakeRotator` 0.0 (+ (* (`self.GetCurrentLeverValue`) -50.0) Value)) false false))

(event `self.ReceiveTick`
  (params (DeltaSeconds :type "Float (single-precision)"))
  (bind _returnvalue_x (`KismetMathLibrary.BreakVector` (`KismetMathLibrary.Quat_VectorForward` (`KismetMathLibrary.Conv_RotatorToQuaternion` (`SceneComponent.RelativeRotation` (`self.HandleMesh`))))))
  (`self.SetLeverValue` (* _returnvalue_x 1.30541)))

(event `self.CalculateLeverRotation`
  (params (GrabberHand :type "SceneComponent Object Reference") (Handle :type "StaticMeshComponent Object Reference"))
  (`SceneComponent.K2_SetRelativeRotation` (`self.HandleMesh`) (`KismetMathLibrary.MakeRotator` 0.0 (`KismetMathLibrary.FClamp` (+ (`KismetMathLibrary.SelectFloat` 0.0 (.pitch (`KismetMathLibrary.FindLookAtRotation` (* (`SceneComponent.RelativeLocation` (`self.HandleMesh`)) (1.0 0.0 1.0)) (* (`KismetMathLibrary.InverseTransformLocation` (`self.GetTransform`) (`SceneComponent.K2_GetComponentLocation` GrabberHand)) (1.0 0.0 1.0))))) 270.0) 220.0 320.0)) false false))

(fn `UserConstructionScript`)