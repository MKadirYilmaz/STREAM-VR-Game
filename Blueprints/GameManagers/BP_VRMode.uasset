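; BP_VRMode is a game manager Blueprint that makes sure an author credit text exists in the level.
; On BeginPlay it looks for a TextRenderActor tagged "Credits" and stores the first valid match in Credits.
; Otherwise it spawns one with centered author credit text, without tagging it or storing it in Credits.
; Tick is disabled and the construction script only calls its parent.
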(event `self.ReceiveBeginPlay`
  (`parent.ReceiveBeginPlay`)
  (bind _outactors (`GameplayStatics.GetAllActorsOfClassWithTag` "/Script/Engine.TextRenderActor" "Credits"))
  (if (> (`KismetArrayLibrary.Array_Length` _outactors) 0)
    (bind _output (`|GetArrayItem` _outactors))
    (`/Engine/EditorBlueprintResources/StandardMacros.IsValid` _output
      (:`Is Valid`
        (set `self.Credits` _output))
      (:`Is Not Valid`
        (bind _returnvalue (`|SpawnActorFromClass` "/Script/Engine.TextRenderActor" (`self.SpawnTransform`) "Undefined" "MultiplyWithRoot" null null :!label _label))
        (bind _textrender (`TextRenderActor.TextRender` _returnvalue))
        (`TextRenderComponent.K2_SetText` _textrender (`|FormatText` "Created by \nMuhammed Kadir Yilmaz"))
        (`TextRenderComponent.SetHorizontalAlignment` _textrender "EHTA_Center")))
    (else
      (goto _label))))

(fn `UserConstructionScript`
  (`parent.UserConstructionScript`))