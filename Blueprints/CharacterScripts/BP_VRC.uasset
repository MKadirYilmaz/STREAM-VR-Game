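; BP_VRC is the VR player Blueprint, handling hand animation, door interaction, camera adjustment and the teleport ring.
; Grab events set CanGrab and IsGrabbing on each hand's animation Blueprint, while other-interaction events grab or release BP_PhysicsDoorSystem handles on hit actors.
; It uses eye-level tracking, offsets CameraRoot for height input and horizontal recentering over FloorLocation, and moves or toggles the teleport ring.
; Ring rotation and Niagara validity coloring are present but unconnected.
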(event `self.GrabbingAnimBlueprint`
  (params (IsRightHand :type Boolean) (IsGrabbing :type Boolean))
  (bind _returnvalue (select `bool` IsRightHand :`false` (`SkeletalMeshComponent.GetAnimInstance` (`self.LeftHandMesh`)) :`true` (`SkeletalMeshComponent.GetAnimInstance` (`self.RightHandMesh`))))
  (if IsRightHand
    (bind _asright_hand_animation_blueprint (cast `/Game/3D_Models/RightHandAnimationBlueprint` _returnvalue))
    (set `/Game/3D_Models/RightHandAnimationBlueprint.IsGrabbing` IsGrabbing _asright_hand_animation_blueprint)
    (else
      (bind _asleft_hand_animation_blueprint (cast `/Game/3D_Models/LeftHandAnimationBlueprint` _returnvalue))
      (set `/Game/3D_Models/LeftHandAnimationBlueprint.IsGrabbing` IsGrabbing _asleft_hand_animation_blueprint))))

(event `self.CanGrabAnimBlueprint`
  (params (IsRightHand :type Boolean) (CanGrab :type Boolean))
  (bind _returnvalue (select `bool` IsRightHand :`false` (`SkeletalMeshComponent.GetAnimInstance` (`self.LeftHandMesh`)) :`true` (`SkeletalMeshComponent.GetAnimInstance` (`self.RightHandMesh`))))
  (if IsRightHand
    (bind _asright_hand_animation_blueprint (cast `/Game/3D_Models/RightHandAnimationBlueprint` _returnvalue))
    (set `/Game/3D_Models/RightHandAnimationBlueprint.bCanGrab` CanGrab _asright_hand_animation_blueprint)
    (else
      (bind _asleft_hand_animation_blueprint (cast `/Game/3D_Models/LeftHandAnimationBlueprint` _returnvalue))
      (set `/Game/3D_Models/LeftHandAnimationBlueprint.bCanGrab` CanGrab _asleft_hand_animation_blueprint))))

(event `self.OtherInteractionSystems`
  (params (HandIndex :type Integer) (RaycastPoint :type "SceneComponent Object Reference") (OtherInteractionResult :type "HitResult Structure"))
  (bind _asbp_physics_door_system (cast `/Game/Blueprints/Interactables/BP_PhysicsDoorSystem` (`.HitActor` (`GameplayStatics.BreakHitResult` OtherInteractionResult))))
  (`PhysicsDoorSystem.GrabHandle` _asbp_physics_door_system RaycastPoint)
  (`KismetSystemLibrary.PrintString` "GrabbedDoor"))

(event `self.OtherReleaseSystems`
  (params (HandIndex :type Integer) (RaycastPoint :type "SceneComponent Object Reference") (OtherInteractionResult :type "HitResult Structure"))
  (bind _asbp_physics_door_system (cast `/Game/Blueprints/Interactables/BP_PhysicsDoorSystem` (`.HitActor` (`GameplayStatics.BreakHitResult` OtherInteractionResult))))
  (`PhysicsDoorSystem.ReleaseHandle` _asbp_physics_door_system RaycastPoint)
  (`KismetSystemLibrary.PrintString` "ReleasedDoor"))

(event `self.ReceiveTick`
  (params (DeltaSeconds :type "Float (single-precision)")))

(event `ReturnCameraToMiddle`
  (bind (_returnvalue_x _returnvalue_y) (`KismetMathLibrary.BreakVector2D` (- (`KismetMathLibrary.Conv_VectorToVector2D` (`SceneComponent.K2_GetComponentLocation` (`self.FloorLocation`))) (`KismetMathLibrary.Conv_VectorToVector2D` (`SceneComponent.K2_GetComponentLocation` (`self.Camera`))))))
  (`SceneComponent.K2_AddWorldOffset` (`self.CameraRoot`) (`KismetMathLibrary.MakeVector` _returnvalue_x _returnvalue_y) false false))

(event `self.TeleportRingSetup`
  (params (RingLocation :type "Vector Structure") (RingNormal :type "Vector Structure") (CanTeleport :type Boolean))
  (`SceneComponent.K2_SetWorldLocation` (`self.TeleportRing`) RingLocation false false))

(event `self.ReceiveBeginPlay`
  (`HeadMountedDisplayFunctionLibrary.SetTrackingOrigin` "Eye"))

(event `self.SetTeleportRingVisibility`
  (params (bShow :type Boolean))
  (bind _teleportring (`self.TeleportRing`))
  (`ActorComponent.SetActive` _teleportring bShow false)
  (`SceneComponent.SetVisibility` _teleportring bShow false))

(event `InputAxis|VRCameraUp`
  (params (AxisValue :type "Float (single-precision)"))
  (`SceneComponent.K2_AddLocalOffset` (`self.CameraRoot`) (`KismetMathLibrary.MakeVector` 0.0 0.0 AxisValue) false false))

(fn `UserConstructionScript`)