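; Lift actor that sequences its animation montage with the start and end of movement.
; LifterMovingAnim plays the montage unless one is already running, then pauses it at the DoorsClosed notify and enables movement.
; LifterStoppingAnim resumes the paused montage, and completion clears the busy guard for the next trip.
; HighlightPressedButton is an empty event, with its text color logic left disconnected.
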(event `self.LifterMovingAnim`
  (if (`self.MontageFinished`)
    (set `self.MontageFinished` false)
    (bind _notifyname (`|PlayMontage` (`self.LifterMesh`) "/Game/3D_Models/BuildingModels/Lifter/NewLifter/LitferAnimMontage.LitferAnimMontage")
      (:`OnCompleted`
        (set `self.MontageFinished` true))
      (:`OnNotifyBegin`
        (if (== _notifyname "DoorsClosed")
          (`AnimInstance.Montage_Pause` (`SkeletalMeshComponent.GetAnimInstance` (`self.LifterMesh`)) "/Game/3D_Models/BuildingModels/Lifter/NewLifter/LitferAnimMontage.LitferAnimMontage")
          (`self.SetShouldMove` true))))
    (else
      (`KismetSystemLibrary.PrintString` "A Montage Currently Playing"))))

(event `self.LifterStoppingAnim`
  (`AnimInstance.Montage_Resume` (`SkeletalMeshComponent.GetAnimInstance` (`self.LifterMesh`)) "/Game/3D_Models/BuildingModels/Lifter/NewLifter/LitferAnimMontage.LitferAnimMontage"))

(event `self.HighlightPressedButton`
  (params (PressedIndex :type Integer)))

(fn `UserConstructionScript`)