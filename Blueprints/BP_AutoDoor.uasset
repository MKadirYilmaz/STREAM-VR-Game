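; Automatic door actor that opens and closes its skeletal DoorMesh with a single montage.
; Activation plays the montage, pausing at the FullyOpen notify, or flips a closing door back to opening.
; Deactivation starts a delayed recheck that plays the montage in reverse unless the door was reactivated.
; Helper events to start, reverse and resume the montage sit alongside some unconnected test nodes.
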(event `Start Montage`
  (bind _doormesh (`self.DoorMesh`))
  (bind _returnvalue (`SkeletalMeshComponent.GetAnimInstance` _doormesh))
  (bind _notifyname (`|PlayMontage` _doormesh "/Game/3D_Models/BuildingModels/Doors/AutoDoorAnims.AutoDoorAnims")
    (:`OnNotifyBegin`
      (if (== _notifyname "FullyOpen")
        (`AnimInstance.Montage_Pause` _returnvalue "/Game/3D_Models/BuildingModels/Doors/AutoDoorAnims.AutoDoorAnims")
        (`AnimInstance.Montage_SetPlayRate` _returnvalue "/Game/3D_Models/BuildingModels/Doors/AutoDoorAnims.AutoDoorAnims" 1.0)))))

(event `ForceToReverse`
  (`AnimInstance.Montage_SetPlayRate` (`SkeletalMeshComponent.GetAnimInstance` (`self.DoorMesh`)) "/Game/3D_Models/BuildingModels/Doors/AutoDoorAnims.AutoDoorAnims" -1.0))

(event `ResumeMontage`
  (`AnimInstance.Montage_Resume` (`SkeletalMeshComponent.GetAnimInstance` (`self.DoorMesh`)) "/Game/3D_Models/BuildingModels/Doors/AutoDoorAnims.AutoDoorAnims"))

(event `self.ActivateAutoDoor`
  (bind _returnvalue (`SkeletalMeshComponent.GetAnimInstance` (`self.DoorMesh`)))
  (if (`self.IsMontageFinished`)
    (set `self.IsMontageFinished` false)
    (set `self.IsOpening` true)
    (`KismetSystemLibrary.PrintString` "New Montage" true false)
    (bind _notifyname (`|PlayMontage` (`self.DoorMesh`) "/Game/3D_Models/BuildingModels/Doors/AutoDoorAnims.AutoDoorAnims")
      (:`OnCompleted`
        (set `self.IsMontageFinished` true))
      (:`OnNotifyBegin`
        (if (== _notifyname "FullyOpen")
          (`AnimInstance.Montage_Pause` _returnvalue "/Game/3D_Models/BuildingModels/Doors/AutoDoorAnims.AutoDoorAnims")
          (`AnimInstance.Montage_SetPlayRate` _returnvalue "/Game/3D_Models/BuildingModels/Doors/AutoDoorAnims.AutoDoorAnims" 1.0))))
    (elif (not (`self.IsOpening`))
      (`AnimInstance.Montage_SetPlayRate` (`SkeletalMeshComponent.GetAnimInstance` (`self.DoorMesh`)) "/Game/3D_Models/BuildingModels/Doors/AutoDoorAnims.AutoDoorAnims" 1.0) ; Kapaniyorken acmaya calisirsa ilerleyis yonunu dondur
      (set `self.IsOpening` true))))

(event `self.DeactivateAutoDoor`
  (set `self.IsOpening` false)
  (`KismetSystemLibrary.K2_SetTimerDelegate` (delegate `RecheckZone`) 3.0))

(event `RecheckZone`
  (bind _returnvalue (`SkeletalMeshComponent.GetAnimInstance` (`self.DoorMesh`)))
  (if (`self.IsOpening`)
    (`KismetSystemLibrary.PrintString` "Can't close" true false)
    (else
      (`AnimInstance.Montage_SetPlayRate` _returnvalue "/Game/3D_Models/BuildingModels/Doors/AutoDoorAnims.AutoDoorAnims" -1.0)
      (`AnimInstance.Montage_Resume` _returnvalue "/Game/3D_Models/BuildingModels/Doors/AutoDoorAnims.AutoDoorAnims")
      (`KismetSystemLibrary.PrintString` "Closing" true false))))

(event `self.ReceiveTick`
  (params (DeltaSeconds :type "Float (single-precision)")))

(fn `UserConstructionScript`)