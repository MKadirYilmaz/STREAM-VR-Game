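; Base actor for a writable painting surface, such as a board, that takes pen strokes in six colors.
; CreateCustomRenderTargets2D builds a cleared render target per color and binds each to its named texture parameter on BoardMaterial.
; Draw sets the pen material's DrawLocation, then draws that material into the render target selected by color index.
; BeginPlay is empty, and neither material is created here.
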(event `self.CreateCustomRenderTargets2D`
  (for _ (range 6)
    (bind _returnvalue (`KismetRenderingLibrary.CreateRenderTarget2D` 1024 1024))
    (`KismetRenderingLibrary.ClearRenderTarget2D` _returnvalue)
    (`KismetArrayLibrary.Array_Add` (`self.RenderTargets`) _returnvalue)
    (for (_array_element _array_index) (`self.RenderTargets`)
      (switch `int` _array_index
        (:`0`
          (set `self.TextureParamName` "BlackRenderTarget"))
        (:`1`
          (set `self.TextureParamName` "RedRenderTarget"))
        (:`2`
          (set `self.TextureParamName` "BlueRenderTarget"))
        (:`3`
          (set `self.TextureParamName` "GreenRenderTarget"))
        (:`4`
          (set `self.TextureParamName` "YellowRenderTarget"))
        (:`5`
          (set `self.TextureParamName` "PinkRenderTarget")))
      (`MaterialInstanceDynamic.SetTextureParameterValue` (`self.BoardMaterial`) (`self.TextureParamName`) _array_element))))

(event `Draw`
  (params (DrawToLocation :type "Vector2D Structure") (`Color Index` :type Integer))
  (bind _output (`|GetArrayItem` (`self.RenderTargets`) `Color Index`))
  (`|ExecutionSequence`
    (:`then_0`
      (`MaterialInstanceDynamic.SetVectorParameterValue` (`self.PenMaterial`) "DrawLocation" (`KismetMathLibrary.Conv_VectorToLinearColor` (`KismetMathLibrary.Conv_Vector2DToVector` DrawToLocation 0.1))))
    (:`then_1`
      (`/Engine/EditorBlueprintResources/StandardMacros.IsValid` _output
        (:`Is Valid`
          (`KismetRenderingLibrary.DrawMaterialToRenderTarget` _output (`self.PenMaterial`)))
        (:`Is Not Valid`
          (`KismetSystemLibrary.PrintString` "Render Target Is Missing"))))))

(event `self.ReceiveBeginPlay`)

(fn `UserConstructionScript`)