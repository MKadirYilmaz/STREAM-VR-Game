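; BP_HoldablePen is a pen for the painting minigame whose visible color follows the color index on its paint component.
; The construction script creates a dynamic material instance from the PenColor material and applies it to the mesh's second material slot.
; It sets the PenColor parameter to black, red, blue or green based on that index.
; The event graph adds no behavior beyond parent calls.
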(event `self.ReceiveBeginPlay`
  (`parent.ReceiveBeginPlay`))

(event `self.ReceiveTick`
  (params (DeltaSeconds :type "Float (single-precision)"))
  (`parent.ReceiveTick` DeltaSeconds))

(fn `UserConstructionScript`
  (`parent.UserConstructionScript`)
  (bind _returnvalue (`KismetMaterialLibrary.CreateDynamicMaterialInstance` "/Game/Materials/MiniGamesMaterials/PaintingSystem/Originals/PenColor.PenColor"))
  (set `self.PenColorMaterial` _returnvalue)
  (`PrimitiveComponent.SetMaterial` (`self.Mesh`) 1 _returnvalue)
  (`MaterialInstanceDynamic.SetVectorParameterValue` (`self.PenColorMaterial`) "PenColor" (select `int` (`PaintComponent.PenColorIndex` (`self.BP_PaintComponent`)) :`0` (struct) :`1` (struct :`R` 1.0 :`A` 1.0) :`2` (struct :`B` 1.0 :`A` 1.0) :`3` (struct :`G` 1.0 :`A` 1.0) :!type "LinearColor Structure")))