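; Physics item actor for a minigame that can be rewound through a BPTimeRewinder.
; Three events drive it: RewindMode prepares the rewind, StartRewind scrubs a clamped 0–1 index by scaled input while rewinding, and ExecRewind resets the index to full and executes the rewind.
; The actor only forwards calls and tracks the index; the rewinder does the rewind work.
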(event `RewindMode`
  (`TimeRewinder.PrepareRewind` (`self.BP_TimeRewinder`)))

(event `StartRewind`
  (params (IndexValue :type "Float (single-precision)") (DeltaTime :type "Float (single-precision)"))
  (bind _returnvalue (`KismetMathLibrary.FClamp` (+ (`self.CurrentIndex`) (* IndexValue 0.005))))
  (set `self.CurrentIndex` _returnvalue)
  (if (`TimeRewinder.GetIsRewinding` (`self.BP_TimeRewinder`))
    (`TimeRewinder.StartRewind` (`self.BP_TimeRewinder`) _returnvalue DeltaTime)))

(event `ExecRewind`
  (set `self.CurrentIndex` 1.0)
  (`TimeRewinder.ExecuteRewind` (`self.BP_TimeRewinder`)))

(fn `UserConstructionScript`
  (`parent.UserConstructionScript`))