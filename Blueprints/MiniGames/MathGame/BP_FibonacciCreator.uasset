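; BP_FibonacciCreator is a math minigame Blueprint that displays the current Fibonacci number and its index as in-world text.
; The RefreshText event calls Refresh, which writes an index label to TextRender and the 64-bit value to FibonacciTextRender.
; Both values come from getter functions defined outside these graphs, so the Blueprint handles only presentation, with BeginPlay and Tick unused.
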(event `self.RefreshText`
  (`self.Refresh`))

(fn `Refresh`
  (`TextRenderComponent.K2_SetText` (`self.TextRender`) (`KismetTextLibrary.Conv_StringToText` (`KismetStringLibrary.Concat_StrStr` (`KismetStringLibrary.Conv_Int64ToString` (`self.GetCurrentFibonacciIndex`)) ". Fibonacci Number: ")))
  (`TextRenderComponent.K2_SetText` (`self.FibonacciTextRender`) (`KismetTextLibrary.Conv_Int64ToText` (`self.GetCurrentFibonacci`))))