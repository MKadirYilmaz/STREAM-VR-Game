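; Laser shooter actor for the math minigame that briefly stretches a beam mesh toward a target bomb when fired.
; BeginPlay creates a dynamic material for the beam, starting blue, and records the mesh's distance from the Scene component as a scale reference.
; FireLaser scales the beam's Z by bomb distance over that reference and colors it blue or red by button index.
; After a short delay, Z scale is set to the reference value itself.
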(event `self.ReceiveBeginPlay`
  (bind _returnvalue (`PrimitiveComponent.CreateDynamicMaterialInstance` (`self.LaserBeamMesh`) 0 "/Game/3D_Models/MathMiniGame/LaserMaterial.LaserMaterial" "None"))
  (bind _output_get (set `self.LaserMaterial` _returnvalue))
  (`PrimitiveComponent.SetMaterial` (`self.LaserBeamMesh`) 0 _output_get)
  (`MaterialInstanceDynamic.SetVectorParameterValue` _output_get "LaserColor" (`self.Blue`))
  (set `self.InitialLaserScale` (`KismetMathLibrary.Vector_Distance` (`SceneComponent.K2_GetComponentLocation` (`self.LaserBeamMesh`)) (`SceneComponent.K2_GetComponentLocation` (`self.Scene`)))))

(event `self.ReceiveTick`
  (params (DeltaSeconds :type "Float (single-precision)")))

(event `self.FireLaser`
  (params (ButtonIndex :type Integer))
  (bind _laserbeammesh (`self.LaserBeamMesh`))
  (bind _targetbomb (`self.TargetBomb`))
  (`/Engine/EditorBlueprintResources/StandardMacros.IsValid` _targetbomb
    (:`Is Valid`
      (`SceneComponent.SetWorldScale3D` _laserbeammesh (`KismetMathLibrary.MakeVector` 0.05 0.05 (/ (`KismetMathLibrary.Vector_Distance` (`SceneComponent.K2_GetComponentLocation` _laserbeammesh) (`self.K2_GetActorLocation` _targetbomb)) (`self.InitialLaserScale`))))
      (`MaterialInstanceDynamic.SetVectorParameterValue` (`self.LaserMaterial`) "LaserColor" (select `int` ButtonIndex :`0` (`self.Blue`) :`1` (`self.Red`)))
      (`KismetSystemLibrary.Delay` 0.4)
      (`SceneComponent.SetWorldScale3D` (`self.LaserBeamMesh`) (`KismetMathLibrary.MakeVector` 0.05 0.05 (`self.InitialLaserScale`))))))

(fn `UserConstructionScript`)