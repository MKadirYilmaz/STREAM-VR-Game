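; BP_MathScreenSystem is the in-world screen of the math minigame, showing an expression, two answer buttons, health, score and duration.
; Setter events write values into text render components, rounding score and duration to at most one decimal, and SetupTexts triggers a text resize.
; RecalculateWordSizes scales world size from measured local Y extent, fitting the expression alone and each button against both buttons' combined extent.
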(event `self.ReceiveTick`
  (params (DeltaSeconds :type "Float (single-precision)")))

(event `self.SetupTexts`
  (params (Expression :type String) (Button1 :type String) (Button2 :type String))
  (`TextRenderComponent.K2_SetText` (`self.ExpressionRenderer`) (`KismetTextLibrary.Conv_StringToText` Expression))
  (`TextRenderComponent.K2_SetText` (`self.Button1Renderer`) (`KismetTextLibrary.Conv_StringToText` Button1))
  (`TextRenderComponent.K2_SetText` (`self.Button2Renderer`) (`KismetTextLibrary.Conv_StringToText` Button2))
  (`self.RecalculateTextSizes`))

(event `self.SetHealth`
  (params (Health :type Integer))
  (`TextRenderComponent.K2_SetText` (`self.HealthRenderer`) (`KismetTextLibrary.Conv_StringToText` (`KismetStringLibrary.Concat_StrStr` "Health: " (`KismetStringLibrary.Conv_IntToString` Health)))))

(event `self.SetScore`
  (params (Score :type "Float (single-precision)"))
  (`TextRenderComponent.K2_SetText` (`self.ScoreRenderer`) (`KismetTextLibrary.Conv_StringToText` (`KismetStringLibrary.Concat_StrStr` "Score: " (`KismetTextLibrary.Conv_TextToString` (`KismetTextLibrary.Conv_DoubleToText` Score "HalfToEven" false true 1 324 0 1))))))

(event `self.SetDuration`
  (params (Duration :type "Float (single-precision)"))
  (`TextRenderComponent.K2_SetText` (`self.RemainedDuration`) (`KismetTextLibrary.Conv_StringToText` (`KismetStringLibrary.Concat_StrStr` "Duration: " (`KismetTextLibrary.Conv_TextToString` (`KismetTextLibrary.Conv_DoubleToText` Duration "HalfToEven" false true 1 324 0 1))))))

(fn `RecalculateWordSizes`
  (bind _button1renderer (`self.Button1Renderer`))
  (bind _button2renderer (`self.Button2Renderer`))
  (bind _expressionrenderer (`self.ExpressionRenderer`))
  (bind (_returnvalue_x _returnvalue_y) (`KismetMathLibrary.BreakVector` (`TextRenderComponent.GetTextLocalSize` _button1renderer)))
  (bind (_returnvalue_x_2 _returnvalue_y_2) (`KismetMathLibrary.BreakVector` (`TextRenderComponent.GetTextLocalSize` _button2renderer)))
  (bind (_returnvalue_x_3 _returnvalue_y_3) (`KismetMathLibrary.BreakVector` (`TextRenderComponent.GetTextLocalSize` _expressionrenderer)))
  (bind _returnvalue (/ 150.0 (+ _returnvalue_y _returnvalue_y_2)))
  (`|ExecutionSequence`
    (:`then_0`
      (`TextRenderComponent.SetWorldSize` _expressionrenderer (* (`TextRenderComponent.WorldSize` _expressionrenderer) (/ 90.0 _returnvalue_y_3))))
    (:`then_1`
      (`TextRenderComponent.SetWorldSize` _button1renderer (* (`TextRenderComponent.WorldSize` _button1renderer) _returnvalue)))
    (:`then_2`
      (`TextRenderComponent.SetWorldSize` _button2renderer (* (`TextRenderComponent.WorldSize` _button2renderer) _returnvalue)))))

(fn `UserConstructionScript`)