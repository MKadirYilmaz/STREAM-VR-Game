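; Blueprint side of the math mini-game system, handling number display, score reporting and music.
; TextConversion formats values into display text, and AutoSaveSystem passes the score to ScoreShower as the last score.
; MusicSystem crossfades between the spawned game music and the world ambient sound as play starts and stops.
; Leaderboard save and scoreboard update nodes are present but disconnected, so scores are not saved to a slot here.
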(event `self.ReceiveBeginPlay`)

(event `self.TextConversion`
  (params (Value :type "Float (single-precision)") (MaxFractionalDigits :type Integer))
  (`self.SetTextFromBlueprint` (`KismetTextLibrary.Conv_DoubleToText` Value "HalfToEven" false true 1 324 0 MaxFractionalDigits)))

(event `self.AutoSaveSystem`
  (params (Score :type "Float (single-precision)"))
  (bind _scoreshower (`self.ScoreShower`))
  (`|ExecutionSequence`
    (:`then_2`
      (`/Engine/EditorBlueprintResources/StandardMacros.IsValid` _scoreshower
        (:`Is Valid`
          (`/Game/Blueprints/MiniGames/LastScoreShower.SetLastScore` _scoreshower Score))))))

(event `self.MusicSystem`
  (params (bStart :type Boolean))
  (bind _musiccomp (`self.MusicComp`))
  (bind _audiocomponent (`AmbientSound.AudioComponent` (`self.WorldAmbientSound`)))
  (bind _audiocomponent_2 (`AmbientSound.AudioComponent` (`self.WorldAmbientSound`)))
  (if bStart
    (bind _returnvalue (`GameplayStatics.SpawnSound2D` "/Game/MySoundFX/MiniGames/Rush_Hour_Cut_60_Cue.Rush_Hour_Cut_60_Cue" 0.3 1.0 0.0 null))
    (bind _output_get (set `self.MusicComp` _returnvalue))
    (`AudioComponent.FadeIn` _output_get 1.0 0.5 0.0 "Linear")
    (`/Engine/EditorBlueprintResources/StandardMacros.IsValid` _audiocomponent_2
      (:`Is Valid`
        (`AudioComponent.FadeOut` _audiocomponent_2 1.0 0.0 "Linear")))
    (else
      (`/Engine/EditorBlueprintResources/StandardMacros.IsValid` _musiccomp
        (:`Is Valid`
          (`AudioComponent.FadeOut` _musiccomp 1.0 0.0 "Linear")
          (`/Engine/EditorBlueprintResources/StandardMacros.IsValid` _audiocomponent
            (:`Is Valid`
              (`AudioComponent.FadeIn` _audiocomponent 0.0 1.0 0.0 "Linear"))))))))

(fn `UserConstructionScript`)