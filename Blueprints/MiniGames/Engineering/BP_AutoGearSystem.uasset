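; Gear-shift helper for the Engineering minigame that moves a gearbox mesh between three gear positions.
; SetProperties stores the mesh and a location for each of the three gears.
; Three events, one per gear, instantly set the mesh's relative location to the stored position, without sweep or interpolation.
; It has no active BeginPlay or Tick logic, and nothing in the file triggers the shifts.
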(event `self.GearBoxToOne`
  (`SceneComponent.K2_SetRelativeLocation` (`self.GearboxMesh`) (`self.Gear1Location`) false false))

(event `self.GearBoxToTwo`
  (`SceneComponent.K2_SetRelativeLocation` (`self.GearboxMesh`) (`self.Gear2Location`) false false))

(event `self.GearBoxToThree`
  (`SceneComponent.K2_SetRelativeLocation` (`self.GearboxMesh`) (`self.Gear3Location`) false false))

(fn `SetProperties`
  (params (Mesh :type "StaticMeshComponent Object Reference") (Gear1 :type "Vector Structure") (Gear2 :type "Vector Structure") (Gear3 :type "Vector Structure"))
  (set `self.GearboxMesh` Mesh)
  (set `self.Gear1Location` Gear1)
  (set `self.Gear2Location` Gear2)
  (set `self.Gear3Location` Gear3))