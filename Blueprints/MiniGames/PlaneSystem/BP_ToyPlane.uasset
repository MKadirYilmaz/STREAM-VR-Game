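; Flyable toy plane for a minigame, handling engine audio, view transitions and race readouts.
; Tick scales motor sound pitch and volume by speed and refreshes speed and time text; despite its name, TextsLookAtCamera never rotates the text.
; Camera blends alternately enable and disable CameraTransition, which lets Tick offset the camera root toward its default location and VRCameraUp shift it vertically during flight.
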(event `self.ReceiveBeginPlay`
  (bind _returnvalue (`GameplayStatics.SpawnSoundAttached` "/Game/MySoundFX/MiniGames/PlaneEngineSFXCue.PlaneEngineSFXCue" (`self.MotorMesh`) "None" (0.0 0.0 0.0) (struct) "KeepRelativeOffset" false 0.25 1.0 0.0 null null false))
  (bind _output_get (set `self.SoundComp` _returnvalue))
  (`AudioComponent.Stop` _output_get))

(event `self.ReceiveTick`
  (params (DeltaSeconds :type "Float (single-precision)"))
  (bind _returnvalue (`self.GetPlaneCurrentSpeed`))
  (bind _soundcomp (`self.SoundComp`))
  (`AudioComponent.SetPitchMultiplier` _soundcomp (/ _returnvalue 1750.0))
  (`AudioComponent.SetVolumeMultiplier` _soundcomp (/ _returnvalue 2000.0))
  (`self.TextsLookAtCamera`)
  (if (and (`self.CameraTransition`) (`self.GetFlightStarted`))
    (`SceneComponent.K2_AddWorldOffset` (`self.PlaneCameraRoot`) (- (`SceneComponent.K2_GetComponentLocation` (`self.DefaultCameraLoc`)) (`SceneComponent.K2_GetComponentLocation` (`self.PlaneCamera`))) false false)))

(event `self.SoundSystem`
  (params (bStart :type Boolean))
  (bind _soundcomp (`self.SoundComp`))
  (if bStart
    (`AudioComponent.Play` _soundcomp 0.0)
    (else
      (`AudioComponent.Stop` _soundcomp))))

(event `self.TransitionToCamera`
  (params (TargetCameraActor :type "Actor Object Reference") (PlayerController :type "PlayerController Object Reference"))
  (`PlayerController.SetViewTargetWithBlend` PlayerController TargetCameraActor 1.5 "VTBlend_Linear" 0.0 false)
  (`KismetSystemLibrary.Delay` 1.5)
  (`/Engine/EditorBlueprintResources/StandardMacros.FlipFlop`
    (:`A`
      (set `self.CameraTransition` true))
    (:`B`
      (set `self.CameraTransition` false)
      (`SceneComponent.SetVisibility` (`self.Warnings`) false false))))

(event `RaceUIShow`
  (params (ShouldShow :type Boolean))
  (`SceneComponent.SetVisibility` (`self.Duration`) ShouldShow false)
  (`SceneComponent.SetVisibility` (`self.SpeedShow`) ShouldShow false))

(event `InputAxis|VRCameraUp`
  (params (AxisValue :type "Float (single-precision)"))
  (if (and (`self.CameraTransition`) (`self.GetFlightStarted`))
    (`SceneComponent.K2_AddLocalOffset` (`self.PlaneCameraRoot`) (`KismetMathLibrary.MakeVector` 0.0 0.0 AxisValue) false false)))

(event `WarnUIShow`
  (params (`Should Show` :type Boolean))
  (`SceneComponent.SetVisibility` (`self.Warnings`) `Should Show` false))

(fn `TextsLookAtCamera`
  (`|ExecutionSequence`
    (:`then_1`
      (if (`self.GetFlightStarted`)
        (`TextRenderComponent.K2_SetText` (`self.SpeedShow`) (`KismetTextLibrary.Conv_DoubleToText` (/ (`self.GetPlaneCurrentSpeed`) 10.0) "HalfToEven" false true 1 324 0 1))
        (`TextRenderComponent.K2_SetText` (`self.Duration`) (`KismetTextLibrary.Conv_DoubleToText` (`self.GetCurrentTime`) "HalfToEven" false true 1 324 0 2))))))

(fn `UserConstructionScript`)