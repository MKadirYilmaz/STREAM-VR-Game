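; Racing manager for the toy plane mini-game, handling the presentation side of route races through event hooks.
; Saved scores go to the current route's ScoreShower as the last score.
; Race UI and return-zone warning toggles are forwarded to the current BP_ToyPlane, which shows them.
; End screen, UI update and UI removal events are empty; older widget and SaveGame leaderboard logic remains disconnected.
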(event `self.AutoSaveScore`
  (params (Score :type "Float (single-precision)"))
  (bind _returnvalue (`self.GetCurrentRoute`))
  (bind _scoreshower (`self.ScoreShower`))
  (`|ExecutionSequence`
    (:`then_2`
      (if (> (`KismetArrayLibrary.Array_Length` _scoreshower) _returnvalue)
        (`/Game/Blueprints/MiniGames/LastScoreShower.SetLastScore` (`|GetArrayItem` _scoreshower _returnvalue) Score)))))

(event `self.PrintEndScreen`
  (params (RaceCompleted :type Boolean)))

(event `self.RaceScreenUI`
  (params (bShow :type Boolean))
  (bind _asbp_toy_plane (cast `/Game/Blueprints/MiniGames/PlaneSystem/BP_ToyPlane` (`self.GetCurrentPlane`)))
  (`/Game/Blueprints/MiniGames/PlaneSystem/BP_ToyPlane.RaceUIShow` _asbp_toy_plane bShow))

(event `self.WarnPlayerReturnZone`
  (params (ShouldWarn :type Boolean))
  (bind _asbp_toy_plane (cast `/Game/Blueprints/MiniGames/PlaneSystem/BP_ToyPlane` (`self.GetCurrentPlane`)))
  (`/Game/Blueprints/MiniGames/PlaneSystem/BP_ToyPlane.WarnUIShow` _asbp_toy_plane ShouldWarn))

(event `self.UpdateRaceScreenUI`
  (params (PlaneSpeed :type "Float (single-precision)") (Time :type "Float (single-precision)")))

(event `self.RemoveAllRacingUIs`)

(fn `UserConstructionScript`)